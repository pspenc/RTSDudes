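; BP_Unit is a game unit Blueprint with an overhead health bar.
; On BeginPlay it casts the HealthBar component's widget to UI_EnemyOverheadHealthBar and assigns itself as that widget's unit.
; The construction script only calls its parent.
; The remaining graph is disconnected leftovers: chase-and-attack movement, player health-bar hiding and runtime spring-arm camera setup, none of which runs.
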(event `Key|C`
  (params (Key :type "Key Structure")))

(event `self.ReceiveBeginPlay`
  (`|ExecutionSequence`
    (:`then_0`
      (bind _asui_enemy_overhead_health_bar (cast `/Game/_Game/UI_EnemyOverheadHealthBar` (`WidgetComponent.GetUserWidgetObject` (`self.HealthBar`))))
      (`/Game/_Game/UI_EnemyOverheadHealthBar.AssignUnit` _asui_enemy_overhead_health_bar self))))

(event `self.ReceiveTick`
  (params (DeltaSeconds :type "Float (single-precision)")))

(fn `UserConstructionScript`
  (`parent.UserConstructionScript`))