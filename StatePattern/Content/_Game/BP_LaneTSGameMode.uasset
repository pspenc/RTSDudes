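; Game mode Blueprint for what appears to be a lane-based game with waves and opposing Player and Enemy teams.
; On BeginPlay it runs the parent logic, then calls PreWave after a short delay.
; GetEndLocationForTeam maps each team to its goal location, with Neutral returning the origin.
; Two events handle the end of a match by opening the WinScreen or LoseScreen level.
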(event `self.ReceiveBeginPlay`
  (`parent.ReceiveBeginPlay`)
  (`KismetSystemLibrary.Delay` 0.2)
  (`self.PreWave`))

(event `self.GoToWinScreen`
  (`GameplayStatics.OpenLevel` "WinScreen"))

(event `self.GoToLoseScreen`
  (`GameplayStatics.OpenLevel` "LoseScreen"))

(fn `GetEndLocationForTeam`
  (params (Team :type "ETeam Enum" :default "Player"))
  (returns (Loc :type "Vector Structure"))
  (return (select `ETeam` Team :`Player` (`self.PlayerGoalLocation`) :`Enemy` (`self.EnemyGoalLocation`))))

(fn `UserConstructionScript`)