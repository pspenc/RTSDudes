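; BP_UnitPlayerController is a player controller that handles the ability slot selection UI, quitting and level loading.
; PresentSlotSelection swaps a valid InterWaveHUD for a new AbilitySlotSelection widget, passing it the new ability and its level.
; Escape quits the game, and an OnDestroyed handler, with no binding shown here, opens StatePatternMap.
; Tick, BeginPlay, WAkeup and Possess are empty, and a movement-input debug print is disconnected.
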(event `self.ReceiveTick`
  (params (DeltaSeconds :type "Float (single-precision)")))

(event `WAkeup`)

(event `self.ReceivePossess`
  (params (PossessedPawn :type "Pawn Object Reference")))

(event `OnDestroyed_Event_0`
  (params (DestroyedActor :type "Actor Object Reference"))
  (`GameplayStatics.OpenLevel` "StatePatternMap"))

(event `Key|Escape`
  (params (Key :type "Key Structure"))
  (:`Pressed`
    (`KismetSystemLibrary.QuitGame` self "Quit")))

(event `self.PresentSlotSelection`
  (params (NewAbility :type Name) (NewAbilityLevel :type Integer))
  (bind _interwavehud (`self.InterWaveHUD`)
    (:`then`
      (`Widget.RemoveFromParent` _interwavehud)
      (bind _returnvalue (`|CreateWidget` "/Game/_Game/UI/AbilitySlotSelection.AbilitySlotSelection_C" self NewAbility NewAbilityLevel))
      (`UserWidget.AddToViewport` _returnvalue 0))
    (:`else`)))

(fn `UserConstructionScript`)